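; Level manager for a memory card game that deals sprite pairs and tracks tries until all cards are matched.
; BeginPlay creates hidden end-of-level widgets, gathers BP_Card actors and randomly deals paired sprites by drawing from a shrinking array.
; Tick resolves clicked pairs stored in BP_GameInstance after a delay, destroying matches or flipping mismatches back.
; An empty card list flags the level passed and shows NextLevel, or LevelsDone on Level4.
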(event `self.ReceiveBeginPlay`
  (bind _gameinstance (`self.GameInstance`))
  (bind _spritesarray (`self.SpritesArray`))
  (bind _asbp_game_instance (cast `/Game/BP/BP_GameInstance` (`GameplayStatics.GetGameInstance`)))
  (set `self.GameInstance` _asbp_game_instance)
  (bind _returnvalue (`|CreateWidget` "/Game/BP/HUD/NextLevel.NextLevel_C" (`GameplayStatics.GetPlayerController` 0)))
  (bind _output_get (set `self.NextLevelRef` _returnvalue))
  (`UserWidget.AddToViewport` _returnvalue 0)
  (`UserWidget.AddToViewport` _output_get 0)
  (`Widget.SetVisibility` _output_get "Hidden")
  (bind _returnvalue_2 (`|CreateWidget` "/Game/BP/HUD/LevelsDone.LevelsDone_C" (`GameplayStatics.GetPlayerController` 0)))
  (bind _output_get_2 (set `self.LevelsDone` _returnvalue_2))
  (`UserWidget.AddToViewport` _output_get_2 0)
  (`Widget.SetVisibility` _output_get_2 "Hidden")
  (set `/Game/BP/BP_GameInstance.NextLevelRef` (`self.NextLevelRef`) _gameinstance)
  (set `/Game/BP/BP_GameInstance.LevelsDoneRef` _output_get_2 _gameinstance)
  ;[1 1 1] Generating Cards on Map
  (bind _outactors (`GameplayStatics.GetAllActorsOfClass` "/Game/BP/BP_Card.BP_Card_C"))
  (set `self.Cards` _outactors)
  ;[1 1 1] Generate Array of Sprites
  (for (_ _array_index) (`self.Cards`)
    (`KismetArrayLibrary.Array_Add` (`self.SpritesArray`) (`|GetArrayItem` (`self.Sprites`) (mod _array_index (/ (`KismetArrayLibrary.Array_Length` (`self.Cards`)) 2)))))
  ;[1 1 1] Generate Sprites for cards
  (for _array_element (`self.Cards`)
    (bind _output_get_3 (set `self.Random` (`KismetMathLibrary.RandomInteger` (`KismetArrayLibrary.Array_Length` _spritesarray))))
    (set `/Game/BP/BP_Card.Sprite1` (`|GetArrayItem` _spritesarray _output_get_3) _array_element)
    (`KismetArrayLibrary.Array_Remove` (`self.SpritesArray`) (`self.Random`))))

(event `self.ReceiveTick`
  (params (DeltaSeconds :type "Float (single-precision)"))
  (bind _gameinstance (`self.GameInstance`))
  (bind _gameinstance_2 (`self.GameInstance`))
  (bind _gameinstance_3 (`self.GameInstance`))
  (bind _levelsdone (`self.LevelsDone`))
  (bind _nextlevelref (`self.NextLevelRef`))
  (bind _clickedcardssprites (`/Game/BP/BP_GameInstance.ClickedCardsSprites` (`self.GameInstance`)))
  (bind _clickedcards (`/Game/BP/BP_GameInstance.ClickedCards` _gameinstance))
  (bind _clickedcards_2 (`/Game/BP/BP_GameInstance.ClickedCards` _gameinstance_2))
  (if (`KismetArrayLibrary.Array_IsNotEmpty` (`self.Cards`))
    (if (>= (`KismetArrayLibrary.Array_Length` (`/Game/BP/BP_GameInstance.ClickedCardsSprites` (`self.GameInstance`))) 2)
      (if (== (`|GetArrayItem` _clickedcardssprites) (`|GetArrayItem` _clickedcardssprites 1))
        (`KismetSystemLibrary.Delay` 1.0)
        (for _array_element _clickedcards_2
          (`self.K2_DestroyActor` _array_element)
          (`KismetArrayLibrary.Array_Remove` (`self.Cards`))
          (`/Engine/EditorBlueprintResources/StandardMacros.IncrementInt` (`self.WinnedCards`)))
        (`/Engine/EditorBlueprintResources/StandardMacros.IncrementInt` (`self.tries`)
          (:`  `
            (`KismetArrayLibrary.Array_Clear` _clickedcards_2)
            (`KismetArrayLibrary.Array_Clear` (`/Game/BP/BP_GameInstance.ClickedCardsSprites` _gameinstance_2))))
        (else
          (`KismetSystemLibrary.Delay` 1.0)
          (for _array_element_2 _clickedcards
            (`PaperSpriteComponent.SetSprite` (`/Game/BP/BP_Card.CardSprite` _array_element_2) "/Game/Materials/Memo/SpriteClosed1.SpriteClosed1"))
          (`/Engine/EditorBlueprintResources/StandardMacros.IncrementInt` (`self.tries`)
            (:`  `
              (`KismetArrayLibrary.Array_Clear` _clickedcards)
              (`KismetArrayLibrary.Array_Clear` (`/Game/BP/BP_GameInstance.ClickedCardsSprites` _gameinstance)))))))
    (else
      (bind _returnvalue (`GameplayStatics.GetCurrentLevelName` true))
      (if (`KismetStringLibrary.EqualEqual_StrStr` _returnvalue "Level1")
        (set `/Game/BP/BP_GameInstance.Level1Passed` true _gameinstance_3)
        (elif (`KismetStringLibrary.EqualEqual_StrStr` _returnvalue "Level2")
          (set `/Game/BP/BP_GameInstance.Level2Passed` true _gameinstance_3)
          (elif (`KismetStringLibrary.EqualEqual_StrStr` _returnvalue "Level3")
            (set `/Game/BP/BP_GameInstance.Level3Passed` true _gameinstance_3)
            (else
              (set `/Game/BP/BP_GameInstance.Level4Passed` true _gameinstance_3)))))
      (bind _returnvalue_2 (`GameplayStatics.GetCurrentLevelName` true))
      (if (`KismetStringLibrary.EqualEqual_StrStr` _returnvalue_2 "Level4")
        (`Widget.SetVisibility` _levelsdone "Visible")
        (`/Game/BP/HUD/LevelsDone.Update Next Widget` _levelsdone (`self.tries`))
        (else
          (`Widget.SetVisibility` _nextlevelref "Visible")
          (`/Game/BP/HUD/NextLevel.Update Next Widget` _nextlevelref (`self.tries`) 0 0)
          (set `/Game/BP/BP_GameInstance.NextLevelRef` _nextlevelref (`self.GameInstance`)))))))

(fn `RandomArrayGen`
  (bind _cards (`self.Cards`))
  (`KismetMathLibrary.SeedRandomStream` (`self.RandomValue`))
  (for _ _cards
    (for _array_element (`self.RandomArray`)
      (if (== _array_element (`KismetMathLibrary.RandomIntegerInRange` 0 (`KismetArrayLibrary.Array_LastIndex` _cards)))
        (set `self.FlagRandom` true)))
    (if (`self.FlagRandom`)
      _)))

(fn `UserConstructionScript`)