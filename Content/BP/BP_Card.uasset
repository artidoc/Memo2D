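; BP_Card is a clickable card actor for what appears to be a memory matching game, starting with its closed sprite showing.
; On click it reveals its face sprite only if it is closed, fewer than two cards are clicked and the GameInstance's ContMenuRef menu is hidden.
; It then registers itself and its sprite in BP_GameInstance's clicked lists, with no matching or flip-back logic of its own.
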(event `self.ReceiveBeginPlay`
  (`PaperSpriteComponent.SetSprite` (`self.CardSprite`) "/Game/Materials/Memo/SpriteClosed1.SpriteClosed1")
  (bind _asbp_game_instance (cast `/Game/BP/BP_GameInstance` (`GameplayStatics.GetGameInstance`)))
  (set `self.GameInstance` _asbp_game_instance))

(event `self.ReceiveActorOnClicked`
  (params (ButtonPressed :type "Key Structure"))
  (bind _gameinstance (`self.GameInstance`))
  (if (and (< (`KismetArrayLibrary.Array_Length` (`/Game/BP/BP_GameInstance.ClickedCards` (`self.GameInstance`))) 2) (`|EnumEquality` (`Widget.GetVisibility` (`/Game/BP/BP_GameInstance.ContMenuRef` (`self.GameInstance`))) "Hidden") (== (`PaperSpriteComponent.GetSprite` (`self.CardSprite`)) "/Game/Materials/Memo/SpriteClosed1.SpriteClosed1"))
    (`PaperSpriteComponent.SetSprite` (`self.CardSprite`) (`self.Sprite1`))
    (`KismetArrayLibrary.Array_Add` (`/Game/BP/BP_GameInstance.ClickedCardsSprites` _gameinstance) (`self.Sprite1`))
    (`KismetArrayLibrary.Array_Add` (`/Game/BP/BP_GameInstance.ClickedCards` _gameinstance) self)))

(fn `UserConstructionScript`)